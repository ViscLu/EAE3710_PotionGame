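; MainCharacterBP is the player character, a sprite-based pawn moved through the Enhanced Input MoveAction.
; Input drives movement along the actor's forward and right vectors and stores a single-axis MoveVector that favors X over Y.
; Each tick, UpdatePlayerRotation flips the Sprite 180 degrees to match the sign of X velocity, keeping its facing at zero.
; GetMoveVector is an unfinished stub with disconnected logic.
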(event `EnhancedInput|/Game/Input/MoveAction`
  (params (ActionValue :type "Vector2D Structure") (ElapsedSeconds :type "Float (double-precision)") (TriggeredSeconds :type "Float (double-precision)") (InputAction :type "InputAction Object Reference" :default "/Game/Input/MoveAction.MoveAction"))
  (:`Triggered`
    (if (!= ActionValue_X 0.0)
      (set `self.moveVector` (`KismetMathLibrary.MakeVector` ActionValue_X))
      (else
        (set `self.moveVector` (`KismetMathLibrary.MakeVector` 0.0 ActionValue_Y))))
    (`self.AddMovementInput` (`self.GetActorForwardVector` self) ActionValue_Y)
    (`self.AddMovementInput` (`self.GetActorRightVector` self) ActionValue_X)))

(event `self.ReceiveTick`
  (params (DeltaSeconds :type "Float (single-precision)"))
  (`self.UpdatePlayerRotation`))

(event `UpdatePlayerRotation`
  (bind _sprite (`self.Sprite`))
  (bind _velocity_x (`KismetMathLibrary.BreakVector` (`MovementComponent.Velocity` (`self.CharacterMovement`))))
  (`/Engine/EditorBlueprintResources/StandardMacros.CompareFloat` _velocity_x
    (:`>`
      (`SceneComponent.K2_SetRelativeRotation` :`self` _sprite))
    (:`<`
      (`SceneComponent.K2_SetRelativeRotation` _sprite (struct :`Yaw` 180.0) false false))))

(fn `Get Move Vector`
  (returns (MoveV :type "Vector Structure")))

(fn `UserConstructionScript`)