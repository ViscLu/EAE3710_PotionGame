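; PotionTable_BP is an interactable potion table that opens the potion screen for the player.
; On interaction it casts the player controller to MyPlayerControllerBP and tells its HUD to show that screen, passing the InventorySystem and PotionBoxInventorySystem inventories.
; A Box overlap shows and hides a widget as actors enter and leave, without filtering which actor overlaps.
; LookAt returns an empty string.
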(event `/Game/Inventory/IInteractInterface.InteractWith`
  (params (PlayerCharacter :type "/Game/Character/CharacterBP/ApothecaryCharacterBP Object Reference"))
  (bind _asmy_player_controller_bp (cast `/Game/GameMain/MyPlayerControllerBP` (`GameplayStatics.GetPlayerController` 0)))
  (`/Game/UMG/PotionUI_PlayerHUD.ShowPotionScreen` (`/Game/GameMain/MyPlayerControllerBP.HUD` _asmy_player_controller_bp) (`self.InventorySystem`) (`self.PotionBoxInventorySystem`)))

(event `self.Box.OnComponentBeginOverlap`
  (params (OverlappedComponent :type "PrimitiveComponent Object Reference") (OtherActor :type "Actor Object Reference") (OtherComp :type "PrimitiveComponent Object Reference") (OtherBodyIndex :type Integer) (bFromSweep :type Boolean) (SweepResult :type "HitResult Structure (by ref)"))
  (`SceneComponent.SetVisibility` (`self.Widget`) true false))

(event `self.Box.OnComponentEndOverlap`
  (params (OverlappedComponent :type "PrimitiveComponent Object Reference") (OtherActor :type "Actor Object Reference") (OtherComp :type "PrimitiveComponent Object Reference") (OtherBodyIndex :type Integer))
  (`SceneComponent.SetVisibility` (`self.Widget`) false false))

(fn `LookAt`
  (returns (Message :type Text))
  (return ""))

(fn `UserConstructionScript`)