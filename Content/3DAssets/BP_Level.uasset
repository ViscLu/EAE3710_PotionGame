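; BP_Level is a level gate that moves the player to another map when they overlap its collision component.
; Any overlap first saves the game mode's timer and gold coins to the "timeSaveData" slot, before the player check.
; For the player pawn, it then passes TeleTag to the game instance as TeleportationTag and opens the level named by LevelName.
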(event `self.LevelGate_Collision.OnComponentBeginOverlap`
  (params (OverlappedComponent :type "PrimitiveComponent Object Reference") (OtherActor :type "Actor Object Reference") (OtherComp :type "PrimitiveComponent Object Reference") (OtherBodyIndex :type Integer) (bFromSweep :type Boolean) (SweepResult :type "HitResult Structure (by ref)"))
  (`self.SaveLevelData`)
  (if (== OtherActor (`GameplayStatics.GetPlayerPawn` 0))
    (bind _ascharacter_game_instance (cast `/Game/characterGameInstance` (`GameplayStatics.GetGameInstance`)))
    (set `/Game/characterGameInstance.TeleportationTag` (`self.TeleTag`) _ascharacter_game_instance)
    (`GameplayStatics.OpenLevel` (`self.LevelName`))))

(fn `SaveLevelData`
  (bind _asmy_game_main_bp (cast `/Game/GameMain/MyGameMainBP` (`GameplayStatics.GetGameMode`)))
  (bind _as_save_data_level_data (`/Game/GameMain/MyGameMainBP.As Save Data Level Data` _asmy_game_main_bp))
  (set `/Game/SaveData_LevelData.MinutesData` (`/Game/GameMain/MyGameMainBP.Minutes` _asmy_game_main_bp) _as_save_data_level_data)
  (set `/Game/SaveData_LevelData.SecondsData` (`/Game/GameMain/MyGameMainBP.Seconds` _asmy_game_main_bp) _as_save_data_level_data)
  (set `/Game/SaveData_LevelData.GoldCoinData` (`/Game/GameMain/MyGameMainBP.GoldCoin` _asmy_game_main_bp) _as_save_data_level_data)
  (`GameplayStatics.SaveGameToSlot` _as_save_data_level_data "timeSaveData"))

(fn `UserConstructionScript`)