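; Player controller that sets up the player's HUD and input for the local player.
; On BeginPlay, only the local controller creates and displays PotionUI_PlayerHUD, prints a debug string and adds the character's Enhanced Input mapping context.
; The OpenBackpack action calls the stored HUD to display the player backpack, while the MoveAction handler is an empty stub.
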(event `self.ReceiveBeginPlay`
  (bind _returnvalue (pcsubsystem `EnhancedInputLocalPlayerSubsystem` self))
  (if (`self.IsLocalController`)
    (bind _returnvalue_2 (`|GenericCreateObject` "/Game/UMG/PotionUI_PlayerHUD.PotionUI_PlayerHUD_C"))
    (bind _output_get (set `self.HUD` _returnvalue_2))
    (`UserWidget.AddToViewport` _output_get 0)
    (`KismetSystemLibrary.PrintString` "666666")
    (`/Engine/EditorBlueprintResources/StandardMacros.IsValid` _returnvalue
      (:`Is Valid`
        (`EnhancedInputSubsystemInterface.AddMappingContext` _returnvalue "/Game/Input/CharacterInputMappingContext.CharacterInputMappingContext" 0 (struct))))))

(event `InputAction|OpenBackpack`
  (params (Key :type "Key Structure"))
  (:`Pressed`
    (`/Game/UMG/PotionUI_PlayerHUD.DisplayPlayerBackpack` (`self.HUD`))))

(event `EnhancedInput|/Game/Input/MoveAction`
  (params (ActionValue :type "Vector2D Structure") (ElapsedSeconds :type "Float (double-precision)") (TriggeredSeconds :type "Float (double-precision)") (InputAction :type "InputAction Object Reference" :default "/Game/Input/MoveAction.MoveAction")))

(fn `UserConstructionScript`)