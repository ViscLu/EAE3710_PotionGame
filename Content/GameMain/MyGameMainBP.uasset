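; Game mode that runs a repeating countdown, tracks gold coins and picks player spawn points.
; BeginPlay loads time and gold from the timeSaveData slot, or creates that save if missing.
; A Delay on Tick steps the timer each second; expiry restarts it and deducts gold, without saving.
; AddGoldCoins saves the new total, and ChoosePlayerStart matches PlayerStart tags to the game instance's TeleportationTag.
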(event `self.ReceiveBeginPlay`
  (bind _returnvalue (`GameplayStatics.DoesSaveGameExist` "timeSaveData"))
  (if _returnvalue
    (bind _returnvalue_2 (`GameplayStatics.LoadGameFromSlot` "timeSaveData"))
    (bind _assave_data_level_data (cast `/Game/SaveData_LevelData` _returnvalue_2))
    (bind _output_get (set `self.As Save Data Level Data` _assave_data_level_data))
    (set `self.Minutes` (`/Game/SaveData_LevelData.MinutesData` _assave_data_level_data))
    (set `self.Seconds` (`/Game/SaveData_LevelData.SecondsData` _assave_data_level_data))
    (set `self.GoldCoin` (`/Game/SaveData_LevelData.GoldCoinData` _assave_data_level_data))
    (`GameplayStatics.SaveGameToSlot` _output_get "timeSaveData")
    (else
      (bind _returnvalue_3 (`GameplayStatics.CreateSaveGameObject` "/Game/SaveData_LevelData.SaveData_LevelData_C"))
      (bind _output_get_2 (set `self.As Save Data Level Data` _returnvalue_3))
      (`GameplayStatics.SaveGameToSlot` _output_get_2 "timeSaveData"))))

(event `self.ReceiveTick`
  (params (DeltaSeconds :type "Float (single-precision)"))
  (`KismetSystemLibrary.Delay` 1.0)
  (if (== (`self.Seconds`) 0)
    (if (== (`self.Minutes`) 0)
      (set `self.Minutes` 2)
      (set `self.GoldCoin` (- (`self.GoldCoin`) 10))
      (else
        (set `self.Seconds` 59)
        (set `self.Minutes` (- (`self.Minutes`) 1))))
    (else
      (set `self.Seconds` (- (`self.Seconds`) 1)))))

(fn `AddGoldCoins`
  (params (addNum :type Integer))
  (set `self.GoldCoin` (+ addNum (`self.GoldCoin`)))
  (bind _returnvalue (`GameplayStatics.LoadGameFromSlot` "timeSaveData"))
  (bind _assave_data_level_data (cast `/Game/SaveData_LevelData` _returnvalue))
  (set `/Game/SaveData_LevelData.GoldCoinData` (`self.GoldCoin`) _assave_data_level_data)
  (`GameplayStatics.SaveGameToSlot` _assave_data_level_data "timeSaveData"))

(fn `ChoosePlayerStart`
  (params (Player :type "Controller Object Reference"))
  (returns (ReturnValue :type "Actor Object Reference"))
  (bind _ascharacter_game_instance (cast `/Game/characterGameInstance` (`GameplayStatics.GetGameInstance`)))
  (bind _outactors (`GameplayStatics.GetAllActorsOfClass` "/Script/Engine.PlayerStart"))
  (for _array_element _outactors
    (if (== (`PlayerStart.PlayerStartTag` _array_element) (`/Game/characterGameInstance.TeleportationTag` _ascharacter_game_instance))
      (return _array_element))))

(fn `UserConstructionScript`)